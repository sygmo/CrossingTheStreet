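; Player character Blueprint for what appears to be a street-crossing game, registering the IMC_CrossingTheStreet Enhanced Input context on BeginPlay.
; Move input drives world-axis movement, independent of camera or facing, and is stored in Directionality.
; Dash launches the character horizontally by scaling current velocity, with delays clearing IsDashing and then restoring CanDash as a cooldown.
; Other inputs quit the game or reset by opening the Sandbox level.
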(event `self.ReceiveBeginPlay`
  (bind _asplayer_controller (cast `PlayerController` (`self.GetController`)))
  (`EnhancedInputSubsystemInterface.AddMappingContext` (pcsubsystem `EnhancedInputLocalPlayerSubsystem` _asplayer_controller) "/Game/Input/IMC_CrossingTheStreet.IMC_CrossingTheStreet" 0 (struct)))

(event `EnhancedInput|/Game/Input/Actions/IA_Move`
  (params (ActionValue :type "Vector2D Structure") (ElapsedSeconds :type "Float (double-precision)") (TriggeredSeconds :type "Float (double-precision)") (InputAction :type "InputAction Object Reference" :default "/Game/Input/Actions/IA_Move.IA_Move"))
  (bind (_x _y) (`KismetMathLibrary.BreakVector2D` ActionValue))
  (:`Triggered`
    (set `self.Directionality` ActionValue)
    (`self.AddMovementInput` (1.0 0.0 0.0) _x)
    (`self.AddMovementInput` (0.0 1.0 0.0) _y)))

(event `EnhancedInput|/Game/Input/Actions/IA_QuitGame`
  (params (ActionValue :type Boolean) (ElapsedSeconds :type "Float (double-precision)") (TriggeredSeconds :type "Float (double-precision)") (InputAction :type "InputAction Object Reference" :default "/Game/Input/Actions/IA_QuitGame.IA_QuitGame"))
  (:`Triggered`
    (`KismetSystemLibrary.QuitGame` null "Quit")))

(event `EnhancedInput|/Game/Input/Actions/IA_ResetLevel`
  (params (ActionValue :type Boolean) (ElapsedSeconds :type "Float (double-precision)") (TriggeredSeconds :type "Float (double-precision)") (InputAction :type "InputAction Object Reference" :default "/Game/Input/Actions/IA_ResetLevel.IA_ResetLevel"))
  (:`Triggered`
    (`GameplayStatics.OpenLevelBySoftObjectPtr` "/Game/MAPS/Sandbox.Sandbox")))

(event `EnhancedInput|/Game/Input/Actions/IA_Dash`
  (params (ActionValue :type Boolean) (ElapsedSeconds :type "Float (double-precision)") (TriggeredSeconds :type "Float (double-precision)") (InputAction :type "InputAction Object Reference" :default "/Game/Input/Actions/IA_Dash.IA_Dash"))
  (bind (_returnvalue_x _returnvalue_y) (`KismetMathLibrary.BreakVector` (* (`self.GetVelocity`) 10.0)))
  (:`Triggered`
    (if (`self.canDash`)
      (set `self.IsDashing` true)
      (set `self.canDash` false)
      (`self.LaunchCharacter` (`KismetMathLibrary.MakeVector` _returnvalue_x _returnvalue_y))
      (`KismetSystemLibrary.Delay` 0.2)
      (set `self.IsDashing` false)
      (`KismetSystemLibrary.Delay` 0.8)
      (set `self.canDash` true))))

(fn `UserConstructionScript`)