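; BP_Vehicle_Base is a base vehicle with a configurable flipbook sprite that travels along a referenced spline and acts as a hazard to the player character.
; On BeginPlay, a timeline scaled by TimeToComplete drives the actor's location and rotation along the spline's length.
; Hurtbox overlap with BP_Char disables its movement and hides it, unless it holds an invincibility item, which is cleared after a short delay.
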(event `self.ReceiveBeginPlay`
  (`self.Move Object`))

(event `Move Object`
  (bind _spline (`/Game/Blueprints/BP_SplinePath.Spline` (`self.SplineReference`)))
  (`TimelineComponent.SetPlayRate` (`self.T_Move`) (/ 1.0 (`self.TimeToComplete`)))
  (bind (_direction _move_track) (`Timeline|T_Move`)
    (:`Update`
      (bind _returnvalue (`KismetMathLibrary.Lerp` 0.0 (`SplineComponent.GetSplineLength` _spline) _move_track))
      (`self.K2_SetActorLocationAndRotation` (`SplineComponent.GetLocationAtDistanceAlongSpline` _spline _returnvalue "World") (`SplineComponent.GetRotationAtDistanceAlongSpline` _spline _returnvalue "World")))))

(event `self.Hurtbox.OnComponentBeginOverlap`
  (params (OverlappedComponent :type "PrimitiveComponent Object Reference") (OtherActor :type "Actor Object Reference") (OtherComp :type "PrimitiveComponent Object Reference") (OtherBodyIndex :type Integer) (bFromSweep :type Boolean) (SweepResult :type "HitResult Structure (by ref)"))
  (bind _asbp_char (cast `/Game/Blueprints/Characters/Character/BP_Char` OtherActor))
  (if (`/Game/Blueprints/Characters/Character/BP_Char.HasInvincibilityItem` _asbp_char)
    (`KismetSystemLibrary.Delay` 1.0)
    (set `/Game/Blueprints/Characters/Character/BP_Char.HasInvincibilityItem` false _asbp_char)
    (else
      (`CharacterMovementComponent.DisableMovement` (`Character.CharacterMovement` _asbp_char))
      (`self.SetActorHiddenInGame` _asbp_char true))))

(fn `UserConstructionScript`
  (`PaperFlipbookComponent.SetFlipbook` (`self.Sprite`) (`self.VehicleSprite`)))